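; Grid manager for a two-sided, turn-based Rebel versus Corporation block game, handling board setup, turns and scores.
; BeginPlay spawns a Block and Rebel_Player at each cell, offsetting cells after the first six along Y.
; Enter swaps sides, recoloring blocks per side, toggling Rebel spheres and updating the HUD, with Corporation points accumulating each turn.
; Enter and Backspace toggle the handover cube and prompts; Backspace also counts turns and shows Rebel health.
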(event Custom|Hide%20Rebel%20Health
  ;[1 1 1] Show/Hide Rebel Health
  (Rendering|SetVisibility (Variables|Default|GetRebelHealth) false false))

(event Custom|SubScore%20Corp
  ;[1 1 1] Handle scoring
  (Variables|Default|SetScore%20Corp (- (Variables|Default|GetScore%20Corp) 1)))

(event Custom|Update%20Corp%20Score
  ;[1 1 1] Handle scoring
  (Variables|Default|SetTotal%20Score%20Corp (+ (Variables|Default|GetTotal%20Score%20Corp) (Variables|Default|GetScore%20Corp)))
  (Rendering|Components|TextRender|SetText (Variables|Default|GetScoreText) (Utilities|Text|ToText(String) (Utilities|String|BuildString(Integer) "" "Points:" (Variables|Default|GetTotal%20Score%20Corp)))))

(event Custom|SubScore%20Reb
  ;[1 1 1] Handle scoring
  (Variables|Default|SetScore%20Rebel (- (Variables|Default|GetScore%20Rebel) 1)))

(event Custom|AddScore%20Corp
  ;[1 1 1] Handle scoring
  (Variables|Default|SetScore%20Corp (+ (Variables|Default|GetScore%20Corp) 1)) ; Update Score
)

(event Custom|AddScore%20Rebel
  ;[1 1 1] Handle scoring
  (Variables|Default|SetScore%20Rebel (+ (Variables|Default|GetScore%20Rebel) 1))
  (Rendering|Components|TextRender|SetText (Variables|Default|GetScoreText) (Utilities|Text|ToText(String) (Utilities|String|BuildString(Integer) "" "Owned:" (Variables|Default|GetScore%20Rebel)))))

(event Custom|Show%20Rebel%20Health
  ;[1 1 1] Show/Hide Rebel Health
  (Rendering|SetVisibility (Variables|Default|GetRebelHealth) true false)
  (Rendering|Components|TextRender|SetText (Variables|Default|GetRebelHealth) (Utilities|Text|ToText(String) (Utilities|String|BuildString(Integer) "" "Rebel Health: " (Variables|Default|GetRebel%20Health)))))

(event EventBeginPlay
  (bind _self self)
  (bind _rebel_loc (Variables|Default|GetRebel_Loc))
  (bind _blockspacing (Variables|Default|GetBlockSpacing))
  (bind _sizex (Variables|Default|GetSizeX))
  (bind _blockarrayt1 (Variables|Default|GetBlockArrayT1))
  ;[1 1 1] Spawn blocks
  (Input|EnableInput (Game|GetPlayerController 0))
  (for _index (range 0 (- (* (Variables|Default|GetSizeX) (Variables|Default|GetSizeY)) 1)) ; Loop to spawn each block
    (if (<= _index 5)
      (bind _transform (CallFunction|TransformNorm _blockspacing _index _sizex))
      (bind _returnvalue (Game|SpawnActorfromClass "/Game/MapBP/Blueprints/Block.Block_C" _transform "Undefined" 0 _self 0)) ; Spawn a  block
      (Utilities|Array|SetArrayElem _blockarrayt1 _index _returnvalue true)
      (bind _returnvalue_2 (Game|SpawnActorfromClass "/Game/MapBP/Blueprints/Rebel_Player.Rebel_Player_C" _transform "Undefined" 0 0))
      (Utilities|Array|SetArrayElem _rebel_loc _index _returnvalue_2 true)
      (else
        (bind _transform_2 (CallFunction|TransformOther _blockspacing _index _sizex))
        (bind _returnvalue_3 (Game|SpawnActorfromClass "/Game/MapBP/Blueprints/Block.Block_C" _transform_2 "Undefined" 0 _self 0)) ; Spawn a  block
        (Utilities|Array|SetArrayElem _blockarrayt1 _index _returnvalue_3 true)
        (bind _returnvalue_4 (Game|SpawnActorfromClass "/Game/MapBP/Blueprints/Rebel_Player.Rebel_Player_C" _transform_2 "Undefined" 0 0))
        (Utilities|Array|SetArrayElem _rebel_loc _index _returnvalue_4 true)))))

(event Input|KeyboardEvents|Backspace
  (params (Key :type Key%20Structure :default "AnyKey"))
  (bind _cube (Variables|Default|GetCube))
  ;[1 1 1] Turn Change on Key
  (:Pressed
    (CallFunction|ShowRebelHealth)
    (if (Variables|Default|GetGridTurn)
      (Variables|Default|SetTurnNum%20Corp (+ (Variables|Default|GetTurnNum%20Corp) 1))
      (else
        (Variables|Default|SetTurnNum%20Reb (+ (Variables|Default|GetTurnNum%20Reb) 1))))
    (Rendering|ToggleVisibility _cube false)
    (Collision|SetCollisionEnabled _cube "NoCollision")
    (Rendering|ToggleVisibility (Variables|Default|GetBackspace) false)
    (Rendering|ToggleVisibility (Variables|Default|GetSwitch) false)
    (Variables|Default|SetTurn%20Over false)))

(event Input|KeyboardEvents|Enter
  (params (Key :type Key%20Structure :default "AnyKey"))
  (bind _cube (Variables|Default|GetCube))
  (bind _rebel_loc (Variables|Default|GetRebel_Loc))
  ;[1 1 1] Turn Change on Key
  (:Pressed
    (CallFunction|HideRebelHealth)
    (Rendering|ToggleVisibility _cube false)
    (Collision|SetCollisionEnabled _cube "QueryAndPhysics")
    (Rendering|ToggleVisibility (Variables|Default|GetBackspace) false)
    (Rendering|ToggleVisibility (Variables|Default|GetSwitch) false)
    (if (Variables|Default|GetGridTurn)
      (for _array_element _rebel_loc
        (if (Variables|/Game/MapBP/Blueprints/Rebel_Player.Rebel_Player_C|GetLast%20Loc _array_element)
          (Default|ShowSphere _array_element)))
      (for _array_element_2 (Variables|Default|GetBlockArrayT1)
        (if (Variables|/Game/MapBP/Blueprints/Block.Block_C|GetIsActive_Rebel _array_element_2)
          (Rendering|Material|SetMaterial (Variables|/Game/MapBP/Blueprints/Block.Block_C|GetBlockMesh _array_element_2) 0 "/Game/Map/Meshes/OrangeMaterial.OrangeMaterial")
          (elif (Variables|/Game/MapBP/Blueprints/Block.Block_C|GetIsActive_RebOther _array_element_2)
            (Rendering|Material|SetMaterial (Variables|/Game/MapBP/Blueprints/Block.Block_C|GetBlockMesh _array_element_2) 0 "/Game/Map/Meshes/BlueMaterial.BlueMaterial")
            (else
              (Rendering|Material|SetMaterial (Variables|/Game/MapBP/Blueprints/Block.Block_C|GetBlockMesh _array_element_2) 0 "/Game/Map/Meshes/BaseMaterial.BaseMaterial"))))
        (Variables|/Game/MapBP/Blueprints/Block.Block_C|SetBlockTurn _array_element_2 false))
      (Rendering|Components|TextRender|SetText (Variables|Default|GetPlayer%20Role) (Utilities|Text|ToText(String) "Rebel"))
      (Rendering|Components|TextRender|SetText (Variables|Default|GetScoreText) (Utilities|Text|ToText(String) (Utilities|String|BuildString(Integer) "" "Owned:" (Variables|Default|GetScore%20Rebel))))
      (Variables|Default|SetGridTurn false)
      (else
        (for _array_element_3 _rebel_loc
          (if (Variables|/Game/MapBP/Blueprints/Rebel_Player.Rebel_Player_C|GetisShowing _array_element_3)
            (Variables|/Game/MapBP/Blueprints/Rebel_Player.Rebel_Player_C|SetLast%20Loc _array_element_3 true)
            (Default|HideSphere _array_element_3)))
        (for _array_element_4 (Variables|Default|GetBlockArrayT1)
          (if (Variables|/Game/MapBP/Blueprints/Block.Block_C|GetIsActive_Corp _array_element_4)
            (Rendering|Material|SetMaterial (Variables|/Game/MapBP/Blueprints/Block.Block_C|GetBlockMesh _array_element_4) 0 "/Game/Map/Meshes/BlueMaterial.BlueMaterial")
            (elif (Variables|/Game/MapBP/Blueprints/Block.Block_C|GetIsActive_CorOther _array_element_4)
              (Rendering|Material|SetMaterial (Variables|/Game/MapBP/Blueprints/Block.Block_C|GetBlockMesh _array_element_4) 0 "/Game/Map/Meshes/OrangeMaterial.OrangeMaterial")
              (else
                (Rendering|Material|SetMaterial (Variables|/Game/MapBP/Blueprints/Block.Block_C|GetBlockMesh _array_element_4) 0 "/Game/Map/Meshes/BaseMaterial.BaseMaterial"))))
          (Variables|/Game/MapBP/Blueprints/Block.Block_C|SetBlockTurn _array_element_4 true))
        (Rendering|Components|TextRender|SetText (Variables|Default|GetPlayer%20Role) (Utilities|Text|ToText(String) "Corporation"))
        (Rendering|Components|TextRender|SetText (Variables|Default|GetScoreText) (Utilities|Text|ToText(String) (Utilities|String|BuildString(Integer) "" "Points:" (Variables|Default|GetTotal%20Score%20Corp))))
        (Variables|Default|SetGridTurn true)
        (CallFunction|UpdateCorpScore)))))

(fn ConstructionScript)

(fn TransformNorm
  (params (Block%20Spacing :type Float%20%28single-precision%29) (Index :type Integer) (Size%20X :type Integer))
  (return (Math|Conversions|ToTransform(Vector) (+ (Math|Vector|MakeVector (* (Math|Integer|%(Integer) Index Size%20X) Block%20Spacing) (* (/ Index Size%20X) Block%20Spacing) 0.0) (Transformation|GetActorLocation)))))

(fn TransformOther
  (params (Block%20Spacing :type Float%20%28single-precision%29) (Index :type Integer) (Size%20X :type Integer))
  (return (Math|Conversions|ToTransform(Vector) (+ (+ (Math|Vector|MakeVector (* (Math|Integer|%(Integer) Index Size%20X) Block%20Spacing) (* (/ Index Size%20X) Block%20Spacing) 0.0) (Transformation|GetActorLocation)) "0,100.000000, 0"))))