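; Clickable grid tile that the Corp and Rebel sides claim in a turn-based territory game, updating scores on its owning grid.
; Clicks end the turn, except early Corp setup picks; BlockTurn selects the acting side.
; Rebels move their location sphere here before claiming; enemy tiles are flagged first, then flipped, leaving them pre-flagged for recapture.
; Materials show ownership, with green hover on unflagged tiles the acting side does not hold.
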(event OnBeginCursorOver(BlockMesh)
  (params (TouchedComponent :type Primitive%20Component%20Object%20Reference))
  ;[1 1 1] Handle block being moused over
  (if (not (Variables|/Game/MapBP/Blueprints/Block_Grid.Block_Grid_C|GetTurn%20Over (Variables|Default|GetOwningGrid)))
    (if (not (Variables|Default|GetIsActive_CorOther))
      (if (not (Variables|Default|GetIsActive_RebOther))
        (if (Variables|Default|GetBlockTurn)
          (if (not (Variables|Default|GetIsActive_Corp)) ; Check we are not already active
            (Rendering|Material|SetMaterial (Variables|Default|GetBlockMesh) 0 "/Game/Map/Meshes/GreenMaterial.GreenMaterial") ; Change material
          )
          (elif (not (Variables|Default|GetIsActive_Rebel)) ; Check we are not already active
            (Rendering|Material|SetMaterial (Variables|Default|GetBlockMesh) 0 "/Game/Map/Meshes/GreenMaterial.GreenMaterial") ; Change material
          ))))))

(event OnClicked(BlockMesh)
  (params (TouchedComponent :type Primitive%20Component%20Object%20Reference))
  (bind _self self)
  (bind _blockmesh (Variables|Default|GetBlockMesh))
  (bind _owninggrid (Variables|Default|GetOwningGrid))
  (bind _owninggrid_2 (Variables|Default|GetOwningGrid))
  (bind _owninggrid_3 (Variables|Default|GetOwningGrid))
  (bind _owninggrid_4 (Variables|Default|GetOwningGrid))
  (bind _blockmesh_2 (Variables|Default|GetBlockMesh))
  (bind _owninggrid_5 (Variables|Default|GetOwningGrid))
  (bind _rebel_loc (Variables|/Game/MapBP/Blueprints/Block_Grid.Block_Grid_C|GetRebel_Loc _owninggrid_2))
  (bind _blockarrayt1 (Variables|/Game/MapBP/Blueprints/Block_Grid.Block_Grid_C|GetBlockArrayT1 _owninggrid_2))
  (bind _returnvalue (Utilities|Array|FindItem _blockarrayt1 _self))
  (bind _item (Utilities|Array|Get(acopy) _rebel_loc _returnvalue))
  ;[1 1 1] Handle block being clicked
  (if (not (Variables|/Game/MapBP/Blueprints/Block_Grid.Block_Grid_C|GetTurn%20Over _owninggrid))
    (if (Variables|/Game/MapBP/Blueprints/Block_Grid.Block_Grid_C|GetGridTurn _owninggrid)
      (if (Variables|/Game/MapBP/Blueprints/Block_Grid.Block_Grid_C|GetSet%20Up _owninggrid)
        (bind _output_get (Variables|/Game/MapBP/Blueprints/Block_Grid.Block_Grid_C|SetCorp%20Num%20Setup _owninggrid_5 (+ (Variables|/Game/MapBP/Blueprints/Block_Grid.Block_Grid_C|GetCorp%20Num%20Setup _owninggrid_5) 1)))
        (if (>= _output_get 3)
          (Variables|/Game/MapBP/Blueprints/Block_Grid.Block_Grid_C|SetTurn%20Over _owninggrid true :!label _label))
        (else
          (goto _label)))
      (else
        (goto _label)))
    (if (Variables|Default|GetBlockTurn)
      (if (Variables|Default|GetIsActive_Rebel)
        (if (Variables|Default|GetIsActive_CorOther)
          (Rendering|Material|SetMaterial _blockmesh 0 "/Game/Map/Meshes/BlueMaterial.BlueMaterial")
          (Default|SubScoreReb _owninggrid_3)
          (Default|AddScoreCorp _owninggrid_3)
          (Variables|Default|SetIsActive_CorOther false)
          (Variables|Default|SetIsActive_RebOther true)
          (Variables|Default|SetIsActive_Corp true)
          (Variables|Default|SetIsActive_Rebel false)
          (else
            (Rendering|Material|SetMaterial _blockmesh 0 "/Game/Map/Meshes/OrangeMaterial.OrangeMaterial")
            (Variables|Default|SetIsActive_CorOther true)))
        (elif (not (Variables|Default|GetIsActive_Corp))
          (Variables|Default|SetIsActive_Corp true)
          (Rendering|Material|SetMaterial (Variables|Default|GetBlockMesh) 0 "/Game/Map/Meshes/BlueMaterial.BlueMaterial")
          (Default|AddScoreCorp (Variables|Default|GetOwningGrid))))
      (elif (Variables|/Game/MapBP/Blueprints/Rebel_Player.Rebel_Player_C|GetisShowing _item)
        (if (Variables|Default|GetIsActive_Corp)
          (if (Variables|Default|GetIsActive_RebOther)
            (Rendering|Material|SetMaterial _blockmesh_2 0 "/Game/Map/Meshes/OrangeMaterial.OrangeMaterial")
            (Default|SubScoreCorp _owninggrid_4)
            (Default|AddScoreRebel _owninggrid_4)
            (Variables|Default|SetIsActive_RebOther false)
            (Variables|Default|SetIsActive_CorOther true)
            (Variables|Default|SetIsActive_Rebel true)
            (Variables|Default|SetIsActive_Corp false)
            (else
              (Rendering|Material|SetMaterial _blockmesh_2 0 "/Game/Map/Meshes/BlueMaterial.BlueMaterial")
              (Variables|Default|SetIsActive_RebOther true)))
          (elif (not (Variables|Default|GetIsActive_Rebel))
            (Variables|Default|SetIsActive_Rebel true)
            (Rendering|Material|SetMaterial (Variables|Default|GetBlockMesh) 0 "/Game/Map/Meshes/OrangeMaterial.OrangeMaterial")
            (Default|AddScoreRebel (Variables|Default|GetOwningGrid))))
        (else
          (for _array_element _rebel_loc
            (Default|HideSphere _array_element)
            (Variables|/Game/MapBP/Blueprints/Rebel_Player.Rebel_Player_C|SetlastLoc _array_element false))
          (Default|ShowSphere _item)
          (Variables|/Game/MapBP/Blueprints/Rebel_Player.Rebel_Player_C|SetlastLoc _item true))))))

(event OnEndCursorOver(BlockMesh)
  (params (TouchedComponent :type Primitive%20Component%20Object%20Reference))
  ;[1 1 1] Handle block being moused over
  (if (not (Variables|/Game/MapBP/Blueprints/Block_Grid.Block_Grid_C|GetTurn%20Over (Variables|Default|GetOwningGrid)))
    (if (not (Variables|Default|GetIsActive_CorOther))
      (if (not (Variables|Default|GetIsActive_RebOther))
        (if (Variables|Default|GetBlockTurn)
          (if (not (Variables|Default|GetIsActive_Corp)) ; Check we are not already active
            (Rendering|Material|SetMaterial (Variables|Default|GetBlockMesh) 0 "/Game/Map/Meshes/BaseMaterial.BaseMaterial") ; Change material
          )
          (elif (not (Variables|Default|GetIsActive_Rebel)) ; Check we are not already active
            (Rendering|Material|SetMaterial (Variables|Default|GetBlockMesh) 0 "/Game/Map/Meshes/BaseMaterial.BaseMaterial") ; Change material
          ))))))

(fn ConstructionScript)